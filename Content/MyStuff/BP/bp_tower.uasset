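; Tower Blueprint that plays status visual effects for marked, frozen and controlled states.
; Each event tints the hit wave effect red, blue or green through its User.Color parameter and activates it.
; The marked state also activates a mark aura effect.
; The Blueprint holds no other logic, as BeginPlay, overlap, Tick and the construction script are empty.
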(event `self.SetMarkedVisuals`
  (`NiagaraComponent.SetVariableLinearColor` (`self.HitWaveEffect`) "User.Color" (make `LinearColor` 20.0 0.0 0.0 1.0))
  (`ActorComponent.Activate` (`self.HitWaveEffect`) false)
  (`ActorComponent.Activate` (`self.MarkAuraEffect`) false))

(event `self.SetFrozenVisuals`
  (`NiagaraComponent.SetVariableLinearColor` (`self.HitWaveEffect`) "User.Color" (make `LinearColor` 0.0 0.0 20.0 1.0))
  (`ActorComponent.Activate` (`self.HitWaveEffect`) false))

(event `self.SetControlledVisuals`
  (`NiagaraComponent.SetVariableLinearColor` (`self.HitWaveEffect`) "User.Color" (make `LinearColor` 0.0 15.0 0.0 1.0))
  (`ActorComponent.Activate` (`self.HitWaveEffect`) false))

(fn `UserConstructionScript`)